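; Fishing rod actor that casts and reels in a BP_FishingLure, linked to the rod's Sphere by a runtime-added cable.
; A physics handle holds the lure until Cast input ends, then an impulse scaled by hold time throws it.
; Tick applies rod rotation and, while ReelingAmount is positive, pulls the landed lure horizontally, then vertically once close, until it is re-grabbed.
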(event `self.ReceiveBeginPlay`
  (bind _sphere (`self.Sphere`))
  ; BEGIN PLAY
  (`self.PickUp`)
  (bind _returnvalue (`GameplayStatics.GetActorOfClass` "/Game/Egging/BP_FishingLure.BP_FishingLure_C"))
  (bind _output_get (set `self.Lure` _returnvalue))
  (`/Engine/EditorBlueprintResources/StandardMacros.IsValid` _output_get
    (:`Is Valid`
      (bind _returnvalue_2 (`AddComponent|NODE_AddCableComponent-0` :`self` _output_get))
      (`PrimitiveComponent.SetMaterial` _returnvalue_2 0 "/Game/Egging/FishLineMat.FishLineMat")
      (set `CableComponent.CableWidth` 7.0 _returnvalue_2)
      (`CableComponent.SetAttachEndToComponent` _returnvalue_2 _sphere "None")
      (`CableComponent.SetAttachEndToComponent` _returnvalue_2 _sphere "None")
      (set `CableComponent.EndLocation` (0.0 0.0 0.0) _returnvalue_2)
      (`SceneComponent.SetVisibility` _returnvalue_2 true true)
      (`PhysicsHandleComponent.GrabComponentAtLocation` (`self.PhysicsHandle`) (`/Game/Egging/BP_FishingLure.Sphere` (`self.Lure`)) "None" (`SceneComponent.K2_GetComponentLocation` _sphere)))))

(event `PickUp`
  ; PICKUP
  (set `self.StartTransform` (`self.GetTransform`)))

(event `MyReelIn`
  (bind _sphere (`/Game/Egging/BP_FishingLure.Sphere` (`self.Lure`)))
  (bind _sphere_2 (`/Game/Egging/BP_FishingLure.Sphere` (`self.Lure`)))
  (bind (_returnvalue_x _returnvalue_y _returnvalue_z) (`KismetMathLibrary.BreakVector` (* (`KismetMathLibrary.GetForwardVector` (`KismetMathLibrary.FindLookAtRotation` (`self.K2_GetActorLocation` (`self.Lure`)) (`SceneComponent.K2_GetComponentLocation` (`self.Sphere`)))) (`self.ReelPower`) (`PrimitiveComponent.GetMass` (`/Game/Egging/BP_FishingLure.Sphere` (`self.Lure`))) (`self.ReelingAmount`))))
  ; MYReelIn
  (`/Engine/EditorBlueprintResources/StandardMacros.IsValid` (`self.Lure`)
    (:`Is Valid`
      (if (`/Game/Egging/BP_FishingLure.bIsLanded` (`self.Lure`))
        (if (`self.bIsReeledIn`)
          (`PrimitiveComponent.SetSimulatePhysics` _sphere true)
          (`PrimitiveComponent.AddImpulse` _sphere (`KismetMathLibrary.MakeVector` 0.0 0.0 _returnvalue_z) "None" false)
          (if (`self.bIsLiftedUp`)
            (set `/Game/Egging/BP_FishingLure.bIsLanded` false (`self.Lure`))
            (`PhysicsHandleComponent.GrabComponentAtLocation` (`self.PhysicsHandle`) (`/Game/Egging/BP_FishingLure.Sphere` (`self.Lure`)) "None" (`SceneComponent.K2_GetComponentLocation` (`self.Sphere`)))
            (`PrimitiveComponent.SetEnableGravity` (`/Game/Egging/BP_FishingLure.Sphere` (`self.Lure`)) true)
            (`PrimitiveComponent.SetSimulatePhysics` (`/Game/Egging/BP_FishingLure.Sphere` (`self.Lure`)) true))
          (else
            (set `self.bIsThrown` false)
            (`PrimitiveComponent.SetEnableGravity` _sphere_2 false)
            (`PrimitiveComponent.SetSimulatePhysics` _sphere_2 true)
            (`PrimitiveComponent.AddImpulse` (`/Game/Egging/BP_FishingLure.Sphere` (`self.Lure`)) (`KismetMathLibrary.MakeVector` _returnvalue_x _returnvalue_y) "None" false)))))))

(event `StopReeling`
  ; STOP REELING
  (if (`self.bIsLiftedUp`)
    _
    (elif (`/Game/Egging/BP_FishingLure.bIsLanded` (`self.Lure`))
      (`PrimitiveComponent.SetSimulatePhysics` (`/Game/Egging/BP_FishingLure.Sphere` (`self.Lure`)) false))))

(event `EnhancedInput|/Game/Input/IA_Cast`
  (params (ActionValue :type Boolean) (ElapsedSeconds :type "Float (double-precision)") (TriggeredSeconds :type "Float (double-precision)") (InputAction :type "InputAction Object Reference" :default "/Game/Input/IA_Cast.IA_Cast"))
  ; IA_CAST
  (:`Triggered`
    (`self.CastRod` ElapsedSeconds))
  (:`Canceled`
    (`self.Throw` :!label _label))
  (:`Completed`
    (goto _label)))

(event `CastRod`
  (params (`Cast Time` :type "Float (double-precision)"))
  ; CAST ROD
  (if (`self.bIsLiftedUp`)
    (if (<= `Cast Time` 3.0)
      (set `self.ThrowRotaiton` (* `Cast Time` -10.0))
      (set `self.CastPower` (`KismetMathLibrary.MapRangeClamped` (`KismetMathLibrary.MapRangeClamped` `Cast Time` 0.0 0.0 (`self.MinAngle`) (`self.MaxAngle`)) (`self.MinAngle`) (`self.MaxAngle`) (`self.ReelMinPower`) (`self.ReelMaxPower`))))))

(event `self.ReceiveTick`
  (params (DeltaSeconds :type "Float (single-precision)"))
  (bind (_returnvalue_x _returnvalue_y _returnvalue_z) (`KismetMathLibrary.BreakVector` (`self.K2_GetActorLocation` (`self.Lure`))))
  (bind (_returnvalue_x_2 _returnvalue_y_2 _returnvalue_z_2) (`KismetMathLibrary.BreakVector` (`SceneComponent.K2_GetComponentLocation` (`self.Sphere`))))
  ; TICK
  (`|ExecutionSequence`
    (:`then_0`
      (if (> (`self.ReelingAmount`) 0.0)
        (`self.MyReelIn`)
        (else
          (`self.StopReeling`))))
    (:`then_1`
      (if (`self.bIsThrown`)
        _
        (elif (`self.bIsLiftedUp`)
          _
          (elif (< (`KismetMathLibrary.Vector_Distance` (`KismetMathLibrary.MakeVector` _returnvalue_x _returnvalue_y) (`KismetMathLibrary.MakeVector` _returnvalue_x_2 _returnvalue_y_2)) 100.0)
            (set `self.bIsReeledIn` true)
            (if (`self.bDoOnce`)
              (if (< (`KismetMathLibrary.Vector_Distance` (`KismetMathLibrary.MakeVector` 0.0 0.0 _returnvalue_z) (`KismetMathLibrary.MakeVector` 0.0 0.0 _returnvalue_z_2)) 2.0)
                (set `self.bIsLiftedUp` true)
                (set `self.bDoOnce` false))
              (else
                (`PrimitiveComponent.SetSimulatePhysics` (`/Game/Egging/BP_FishingLure.Sphere` (`self.Lure`)) false)
                (`KismetSystemLibrary.PrintString` "2")
                (set `self.bDoOnce` true)))))))
    (:`then_2`
      (`self.ApplyRotation`))))

(event `Throw`
  (bind _sphere (`/Game/Egging/BP_FishingLure.Sphere` (`self.Lure`)))
  ; THROW
  (if (`self.bIsLiftedUp`)
    (set `self.bIsThrown` true)
    (set `self.bIsLiftedUp` false)
    (set `self.bIsReeledIn` false)
    (`PhysicsHandleComponent.ReleaseComponent` (`self.PhysicsHandle`))
    (`PrimitiveComponent.SetEnableGravity` _sphere true)
    (`PrimitiveComponent.SetSimulatePhysics` _sphere true)
    (`PrimitiveComponent.AddImpulse` (`/Game/Egging/BP_FishingLure.Sphere` (`self.Lure`)) (* (`KismetMathLibrary.GetForwardVector` (`self.K2_GetActorRotation`)) (* (`self.LureSpeed`) (`self.CastPower`) (`PrimitiveComponent.GetMass` (`/Game/Egging/BP_FishingLure.Sphere` (`self.Lure`)))) -5.0) "None" false)
    (set `self.ThrowRotaiton` (.pitch (.rotation (`self.StartTransform`))))))

(event `ApplyRotation`
  (bind (_returnvalue_x _returnvalue_y) (`KismetMathLibrary.BreakVector2D` (* (`self.RodMoveRotationAmount`) (`self.RodDirection`))))
  (`self.K2_SetActorRotation` (`KismetMathLibrary.MakeRotator` 0.0 (+ (`self.ThrowRotaiton`) _returnvalue_x) _returnvalue_y)))

(fn `UserConstructionScript`)