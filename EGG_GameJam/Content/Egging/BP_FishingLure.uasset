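; Fishing lure for an egg-fishing mechanic, which lands in BP_WaterTest, bobs on a sine wave and hooks eggs.
; Tick lerps the lure toward the rod, or to line length when in water.
; It also randomly spawns an M_BaseEgg that hangs below the lure until picked up.
; A hooked egg steers the lure around the rod in random swim directions; older movement and pulling logic is disconnected.
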(event `self.ReceiveActorBeginOverlap`
  (params (OtherActor :type "Actor Object Reference"))
  (bind _sphere (`self.Sphere`))
  (if (== OtherActor (`self.water`))
    (`PrimitiveComponent.SetEnableGravity` _sphere false)
    (`PrimitiveComponent.SetSimulatePhysics` _sphere false)
    (set `self.IsInWater` true)
    (`/Game/Egging/BP_FishingRod.CalculateLineLenght` (`self.EggRod`))
    (set `self.LureIsInAir` false)))

(event `self.ReceiveTick`
  (params (DeltaSeconds :type "Float (single-precision)"))
  (`|ExecutionSequence`
    (:`then_0`
      ; Bobing
      (`self.UpdateLurePosition` DeltaSeconds)
      (if (`self.IsInWater`)
        (`self.OnWaterBobingAndPos` DeltaSeconds)))
    (:`then_1`
      ; EGG
      (`KismetSystemLibrary.Delay` 0.1)
      (`self.AtemptSpawn`))
    (:`then_2`
      (`self.EggPositionUpdate`))
    (:`then_3`
      (`self.Run_EggAi`))))

(event `Run_EggAi`
  ;[0.151 0.0904 0.06136] Egg AAI
  (`/Engine/EditorBlueprintResources/StandardMacros.IsValid` (`self.Current Egg`)
    (:`Is Valid`
      (if (`self.IsInWater`)
        (`|ExecutionSequence`
          (:`then_0`
            (`KismetSystemLibrary.Delay` (`KismetMathLibrary.RandomFloatInRange` 5.0 15.0))
            (`self.DecideDirection`))
          (:`then_1`
            (`self.Egg_Ai`)))))))

(event `idkclamp`
  (bind (_returnvalue_x _returnvalue_y) (`KismetMathLibrary.BreakVector` (`self.K2_GetActorLocation`)))
  (if (> _returnvalue_x 2600.0)
    (set `self.RandomDirX` 0)))

(event `self.ReceiveBeginPlay`
  (bind _returnvalue (`GameplayStatics.GetActorOfClass` "/Game/Egging/BP_WaterTest.BP_WaterTest_C"))
  (set `self.water` _returnvalue)
  (bind _returnvalue_2 (`GameplayStatics.GetActorOfClass` "/Game/Egging/BP_FishingRod.BP_FishingRod_C"))
  (set `self.EggRod` _returnvalue_2))

(event `Movement`
  (bind (_returnvalue_location _returnvalue_rotation _returnvalue_scale) (`KismetMathLibrary.BreakTransform` (`self.GetTransform`)))
  (bind (_pullmultiplier_x _pullmultiplier_y) (`KismetMathLibrary.BreakVector2D` (`self.PullMultiplier`)))
  (`|ExecutionSequence`
    (:`then_0`
      (`/Engine/EditorBlueprintResources/StandardMacros.Gate` true :!label _label
        (:`Exit`
          _)))
    (:`then_1`
      (`KismetSystemLibrary.Delay` (`KismetMathLibrary.RandomFloatInRange` (`self.MinWaitTime`) (`self.MaxWaitTime`)))
      (`/Engine/EditorBlueprintResources/StandardMacros.DoOnce` false
        (:`Completed`
          (`|ExecutionSequence`
            (:`then_0`
              _)
            (:`then_1`
              (goto _label :!via `Open`)))))))
  (`self.PickRandomDirection`)
  (`self.K2_AddActorWorldOffset` (`KismetMathLibrary.MakeVector` (* (stale `PickRandomDirection` _output_get) (+ _pullmultiplier_x 1.0)) (* (stale `PickRandomDirection` _output_get_2) (+ _pullmultiplier_y 1.0))))
  (if (not (`self.bIsEggOn`))
    (bind _returnvalue (`|SpawnActorFromClass` "/Game/EggBoiling/M_BaseEgg.M_BaseEgg_C" (`KismetMathLibrary.MakeTransform` _returnvalue_location (struct) _returnvalue_scale) "Undefined" "MultiplyWithRoot" null null))
    (`PrimitiveComponent.SetSimulatePhysics` (`/Game/EggBoiling/M_BaseEgg.Sphere` _returnvalue) false)
    (set `self.Current Egg` _returnvalue)
    (set `self.bIsEggOn` true)))

(event `PickRandomDirection`
  (bind _returnvalue (`KismetMathLibrary.RandomIntegerInRange` -1 1))
  (`KismetSystemLibrary.Delay` (`self.StartTime`))
  (bind _output_get (set `self.RandomDirX` _returnvalue))
  (bind _output_get_2 (set `self.RandomDirY` _returnvalue))
  (set `self.StartTime` (`KismetMathLibrary.RandomFloatInRange` (`self.MinWaitTime`) (`self.MaxWaitTime`))))

(event `Pulling`
  (bind (_roddirection_x _roddirection_y) (`KismetMathLibrary.BreakVector2D` (`FishingRod.RodDirection` (`self.EggRod`))))
  (set `self.PullMultiplier` (`KismetMathLibrary.MakeVector2D` (`KismetMathLibrary.Abs` (- (`self.RandomDirX`) _roddirection_x)) (`KismetMathLibrary.Abs` (- (`self.RandomDirY`) _roddirection_y)))))

(event `Bob`
  ; inte klar
  (if (`self.bIsLanded`)
    (if (`self.bIsEggOn`)
      (`self.K2_SetActorRotation` (`KismetMathLibrary.FindLookAtRotation` (`self.K2_GetActorLocation`) (+ (`self.K2_GetActorLocation`) (`KismetMathLibrary.MakeVector` (* (`self.RandomDirX`) 90000000.0) (* (`self.RandomDirY`) 90000000.0)))))
      (else
        (set `RotatingMovementComponent.RotationRate` (struct :`Pitch` 5.0 :`Yaw` 5.0 :`Roll` 5.0) (`self.RotatingMovement`))))
    (else
      (set `RotatingMovementComponent.RotationRate` (struct) (`self.RotatingMovement`)))))

(fn `AtemptSpawn`
  (`/Engine/EditorBlueprintResources/StandardMacros.IsValid` (`self.Current Egg`)
    (:`Is Not Valid`
      (if (`self.IsInWater`)
        (if (`KismetMathLibrary.RandomBoolWithWeight` 0.033333)
          (bind _returnvalue (`|SpawnActorFromClass` "/Game/EggBoiling/M_BaseEgg.M_BaseEgg_C" (`KismetMathLibrary.MakeTransform` (0.0 0.0 0.0)) "Undefined" "MultiplyWithRoot" null null))
          (`PrimitiveComponent.SetSimulatePhysics` (`/Game/EggBoiling/M_BaseEgg.Sphere` _returnvalue) false)
          (set `self.Current Egg` _returnvalue)
          (`KismetSystemLibrary.PrintString` "EggSPAW" true true (struct :`R` 1.0 :`G` 0.284577 :`A` 1.0) 10.0))))))

(fn `DecideDirection`
  (set `self.SwimDirection` (`KismetMathLibrary.MakeVector2D` (`KismetMathLibrary.Conv_IntToDouble` (`KismetMathLibrary.RandomIntegerInRange` 1 2)) (`KismetMathLibrary.Conv_IntToDouble` (`KismetMathLibrary.RandomIntegerInRange` -1 1)))))

(fn `Egg_Ai`
  (bind (_returnvalue_x _returnvalue_y _returnvalue_z) (`KismetMathLibrary.BreakVector` (`self.K2_GetActorLocation`)))
  (bind (_returnvalue_x_2 _returnvalue_y_2) (`KismetMathLibrary.BreakVector2D` (* (`KismetMathLibrary.Normal2D` (`self.SwimDirection`)) (`FishingRod.LineLenght` (`self.EggRod`)) (-1.0 -1.0))))
  (bind _returnvalue (`KismetMathLibrary.VLerp` (`self.K2_GetActorLocation`) (+ (`KismetMathLibrary.MakeVector` _returnvalue_x_2 _returnvalue_y_2 _returnvalue_z) (* (`self.K2_GetActorLocation` (`self.EggRod`)) (1.0 1.0 0.0))) (* (`GameplayStatics.GetWorldDeltaSeconds`) (`self.DirectionChangeSpeed`))))
  (bind (_returnvalue_x_3 _returnvalue_y_3) (`KismetMathLibrary.BreakVector` (- (`self.K2_GetActorLocation` (`self.EggRod`)) _returnvalue)))
  (`self.K2_SetActorLocation` _returnvalue)
  (set `self.CurrentSwimDirection` (`KismetMathLibrary.Normal2D` (`KismetMathLibrary.MakeVector2D` _returnvalue_x_3 _returnvalue_y_3))))

(fn `EggPositionUpdate`
  (`/Engine/EditorBlueprintResources/StandardMacros.IsValid` (`self.Current Egg`)
    (:`Is Valid`
      (bind _returnvalue (`Egg.IsPickedUp` (`self.Current Egg`)))
      (if _returnvalue
        (set `self.Current Egg` null)
        (else
          (`SceneComponent.K2_SetWorldLocation` (`/Game/EggBoiling/M_BaseEgg.Sphere` (`self.Current Egg`)) (+ (`self.K2_GetActorLocation`) (0.0 0.0 -50.0)) false false))))))

(fn `OnWaterBobingAndPos`
  (params (DeltaTime :type "Float (double-precision)"))
  (bind (_returnvalue_x _returnvalue_y _returnvalue_z) (`KismetMathLibrary.BreakVector` (`self.K2_GetActorLocation`)))
  (bind (_returnvalue_x_2 _returnvalue_y_2 _returnvalue_z_2) (`KismetMathLibrary.BreakVector` (`self.K2_GetActorLocation` (`self.water`))))
  (`self.K2_SetActorLocation` (`KismetMathLibrary.MakeVector` _returnvalue_x _returnvalue_y (`KismetMathLibrary.Lerp` _returnvalue_z (+ _returnvalue_z_2 (* (- (`KismetMathLibrary.Sin` (* (`GameplayStatics.GetRealTimeSeconds`) (`self.BobingSpeedZ`))) 3.0) (`self.BobingAmountZ`))) (* DeltaTime (`self.BobingLerpSpeedZ`))))))

(fn `UpdateLurePosition`
  (params (Alpha :type "Float (double-precision)"))
  (bind (_returnvalue_x _returnvalue_y _returnvalue_z) (`KismetMathLibrary.BreakVector` (`self.K2_GetActorLocation`)))
  (bind (_returnvalue_x_2 _returnvalue_y_2) (`KismetMathLibrary.BreakVector` (`self.K2_GetActorLocation` (`self.EggRod`))))
  (bind (_returnvalue_x_3 _returnvalue_y_3) (`KismetMathLibrary.BreakVector` (- (`self.K2_GetActorLocation` (`self.EggRod`)) (`self.K2_GetActorLocation`))))
  (bind (_returnvalue_x_4 _returnvalue_y_4) (`KismetMathLibrary.BreakVector2D` (+ (`KismetMathLibrary.MakeVector2D` _returnvalue_x_2 _returnvalue_y_2) (* (`KismetMathLibrary.Normal2D` (`KismetMathLibrary.MakeVector2D` _returnvalue_x_3 _returnvalue_y_3)) (`FishingRod.LineLenght` (`self.EggRod`)) (-1.0 -1.0)))))
  (if (`self.LureIsInAir`)
    _
    (elif (`self.IsInWater`)
      (`/Engine/EditorBlueprintResources/StandardMacros.IsValid` (`self.Current Egg`)
        (:`Is Not Valid`
          (`self.K2_SetActorLocation` (`KismetMathLibrary.VLerp` (`self.K2_GetActorLocation`) (`KismetMathLibrary.MakeVector` _returnvalue_x_4 _returnvalue_y_4 _returnvalue_z) (* Alpha (`self.PositionUpdateSpeed`))))))
      (else
        ; Reeled In Target Pos
        (`self.K2_SetActorLocation` (`KismetMathLibrary.VLerp` (`self.K2_GetActorLocation`) (+ (`SceneComponent.K2_GetComponentLocation` (`/Game/Egging/BP_FishingRod.Sphere` (`self.EggRod`))) (0.0 0.0 -40.0)) (* (`self.PositionUpdateSpeed`) Alpha)))))))

(fn `UserConstructionScript`)